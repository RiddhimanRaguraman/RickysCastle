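; BP_ChaliceB is an interactable chalice that accepts a gem from the third-person character.
; A sphere overlap toggles player input, so pressing Q checks the character's gem flag.
; On success it copies the character's Mellow mesh, snaps it to the "drop" socket, deequips the character, shows success text and sets BComp.
; A disconnected chain checking BP_ChaliceA completion to lower Bp_poKeela never runs.
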(event OnComponentBeginOverlap(Sphere)
  (params (OverlappedComponent :type Primitive%20Component%20Object%20Reference) (OtherActor :type Actor%20Object%20Reference) (OtherComp :type Primitive%20Component%20Object%20Reference) (OtherBodyIndex :type Integer) (bFromSweep :type Boolean) (SweepResult :type Hit%20Result%20Structure%20%28by%20ref%29))
  (Utilities|Casting|CastToBP_ThirdPersonCharacter OtherActor)
  (Input|EnableInput (Game|GetPlayerController 0)))

(event OnComponentEndOverlap(Sphere)
  (params (OverlappedComponent :type Primitive%20Component%20Object%20Reference) (OtherActor :type Actor%20Object%20Reference) (OtherComp :type Primitive%20Component%20Object%20Reference) (OtherBodyIndex :type Integer))
  (Utilities|Casting|CastToBP_ThirdPersonCharacter OtherActor)
  (Input|DisableInput (Game|GetPlayerController 0)))

(event Input|KeyboardEvents|Q
  (params (Key :type Key%20Structure :default "None"))
  (:Pressed
    (bind _asbp_third_person_character (Utilities|Casting|CastToBP_ThirdPersonCharacter (stale OnComponentBeginOverlap(Sphere) OtherActor)))
    (if (Variables|/Game/ThirdPerson/Blueprints/BP_ThirdPersonCharacter.BP_ThirdPersonCharacter_C|GettoCheckGem _asbp_third_person_character)
      (Components|StaticMesh|SetStaticMesh (Variables|Default|Getmellow) (Variables|/Script/Engine.StaticMeshComponent|GetStaticMesh (Variables|/Game/ThirdPerson/Blueprints/BP_ThirdPersonCharacter.BP_ThirdPersonCharacter_C|Getmellow _asbp_third_person_character)))
      (Transformation|AttachComponentToComponent (Variables|Default|Getmellow) (Variables|Default|GetChalice) "drop" "SnapToTarget" "SnapToTarget" "SnapToTarget" true)
      (Default|Deequip _asbp_third_person_character)
      (Rendering|Components|TextRender|SetText (Variables|Default|GetTextRender) (Variables|Default|GetsucessText))
      (Variables|Default|SetBComp true))))

(fn ConstructionScript)