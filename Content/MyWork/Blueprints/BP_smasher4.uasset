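; BP_smasher4 is a looping smasher hazard that damages the third-person character.
; After a short delay on BeginPlay, a self-calling Loop event uses MoveComponentTo to slide a mesh quickly along negative relative X, then return it more slowly, pausing after each move.
; A Box component's begin overlap casts the other actor to BP_ThirdPersonCharacter and calls its BigSmash with Damage.
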(event OnComponentBeginOverlap(Box)
  (params (OverlappedComponent :type Primitive%20Component%20Object%20Reference) (OtherActor :type Actor%20Object%20Reference) (OtherComp :type Primitive%20Component%20Object%20Reference) (OtherBodyIndex :type Integer) (bFromSweep :type Boolean) (SweepResult :type Hit%20Result%20Structure%20%28by%20ref%29))
  (bind _asbp_third_person_character (Utilities|Casting|CastToBP_ThirdPersonCharacter OtherActor))
  (Default|BigSmash _asbp_third_person_character (Variables|Default|GetDamage)))

(event Custom|loop
  (bind _staticmeshactor_uaid_047c16101bba26da01_1289715068 (Variables|Default|GetStaticMeshActor_UAID_047C16101BBA26DA01_1289715068))
  (bind _staticmeshactor_uaid_047c16101bba26da01_1289715068_2 (Variables|Default|GetStaticMeshActor_UAID_047C16101BBA26DA01_1289715068))
  (bind _relativelocation (Variables|/Script/Engine.SceneComponent|GetRelativeLocation _staticmeshactor_uaid_047c16101bba26da01_1289715068_2))
  (bind _relativelocation_2 (Variables|/Script/Engine.SceneComponent|GetRelativeLocation _staticmeshactor_uaid_047c16101bba26da01_1289715068))
  (Components|MoveComponentTo _staticmeshactor_uaid_047c16101bba26da01_1289715068_2 (Math|Vector|MakeVector (- (.x _relativelocation) 5e+02) (.y _relativelocation) (.z _relativelocation)) (Variables|/Script/Engine.SceneComponent|GetRelativeRotation _staticmeshactor_uaid_047c16101bba26da01_1289715068_2) false false 0.2 false)
  (Utilities|FlowControl|Delay 1.0)
  (Components|MoveComponentTo _staticmeshactor_uaid_047c16101bba26da01_1289715068 (Math|Vector|MakeVector (+ (.x _relativelocation_2) 5e+02) (.y _relativelocation_2) (.z _relativelocation_2)) (Variables|/Script/Engine.SceneComponent|GetRelativeRotation _staticmeshactor_uaid_047c16101bba26da01_1289715068) false false 0.5 false)
  (Utilities|FlowControl|Delay 1.5)
  (CallFunction|Loop))

(event EventBeginPlay
  (Utilities|FlowControl|Delay 1.0)
  (CallFunction|Loop))

(event Collision|EventActorBeginOverlap
  (params (OtherActor :type Actor%20Object%20Reference)))

(event EventTick
  (params (DeltaSeconds :type Float%20%28single-precision%29)))

(fn ConstructionScript)