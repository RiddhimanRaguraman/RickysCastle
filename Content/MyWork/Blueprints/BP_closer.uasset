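; BP_closer is an actor with a Cube that stretches closed and retracts along its Y scale, driven by two overlap triggers.
; Overlapping Closer starts a self-calling delay loop that grows the Cube in small, rapid increments up to a limit.
; Overlapping Opener disables Closer's collision and starts a second loop that shrinks it in larger, slower steps.
; Nothing explicitly cancels the growing loop when shrinking starts.
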(event OnComponentBeginOverlap(closer)
  (params (OverlappedComponent :type Primitive%20Component%20Object%20Reference) (OtherActor :type Actor%20Object%20Reference) (OtherComp :type Primitive%20Component%20Object%20Reference) (OtherBodyIndex :type Integer) (bFromSweep :type Boolean) (SweepResult :type Hit%20Result%20Structure%20%28by%20ref%29))
  (CallFunction|Loop))

(event OnComponentBeginOverlap(opener)
  (params (OverlappedComponent :type Primitive%20Component%20Object%20Reference) (OtherActor :type Actor%20Object%20Reference) (OtherComp :type Primitive%20Component%20Object%20Reference) (OtherBodyIndex :type Integer) (bFromSweep :type Boolean) (SweepResult :type Hit%20Result%20Structure%20%28by%20ref%29))
  (Collision|SetCollisionEnabled (Variables|Default|Getcloser) "NoCollision")
  (CallFunction|Loop2))

(event Custom|loop
  (bind _cube (Variables|Default|GetCube))
  (bind _returnvalue (Transformation|GetRelativeTransform _cube))
  (Utilities|FlowControl|Delay 0.005)
  (if (< (.y (.scale _returnvalue)) 16.0)
    (Transformation|SetRelativeTransform _cube (Math|Transform|MakeTransform (.location _returnvalue) (.rotation _returnvalue) (Math|Vector|MakeVector (.x (.scale _returnvalue)) (+ (.y (.scale _returnvalue)) 0.01) (.z (.scale _returnvalue)))) false false)
    (CallFunction|Loop)))

(event Custom|loop2
  (bind _cube (Variables|Default|GetCube))
  (bind _returnvalue (Transformation|GetRelativeTransform _cube))
  (Utilities|FlowControl|Delay 0.5)
  (if (> (.y (.scale _returnvalue)) 1.0)
    (Transformation|SetRelativeTransform _cube (Math|Transform|MakeTransform (.location _returnvalue) (.rotation _returnvalue) (Math|Vector|MakeVector (.x (.scale _returnvalue)) (- (.y (.scale _returnvalue)) 1.0) (.z (.scale _returnvalue)))) false false)
    (CallFunction|Loop2)))

(event EventBeginPlay)

(event Collision|EventActorBeginOverlap
  (params (OtherActor :type Actor%20Object%20Reference)))

(event EventTick
  (params (DeltaSeconds :type Float%20%28single-precision%29)))

(fn ConstructionScript)