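; BP_upRotate is a rotating obstacle actor that pushes the third-person character back on contact.
; Tick adds a fixed world rotation to the Cylinder each frame, without scaling by delta time.
; Capsule overlap casts the other actor to BP_ThirdPersonCharacter and calls its PushBackForce.
; BeginPlay stores a scaled, reversed Cylinder right vector in SendVector, which this graph never reads.
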(event OnComponentBeginOverlap(Capsule)
  (params (OverlappedComponent :type Primitive%20Component%20Object%20Reference) (OtherActor :type Actor%20Object%20Reference) (OtherComp :type Primitive%20Component%20Object%20Reference) (OtherBodyIndex :type Integer) (bFromSweep :type Boolean) (SweepResult :type Hit%20Result%20Structure%20%28by%20ref%29))
  (bind _asbp_third_person_character (Utilities|Casting|CastToBP_ThirdPersonCharacter OtherActor))
  (Default|PushBackForce _asbp_third_person_character))

(event EventBeginPlay
  (Variables|Default|SetsendVector (* (* (Math|Vector|GetRightVector (Variables|Default|Getcylinder)) -1.0) 2.0)))

(event EventTick
  (params (DeltaSeconds :type Float%20%28single-precision%29))
  (Transformation|AddWorldRotation (Variables|Default|Getcylinder) "0.000000,2.000000,0.000000" false false))

(fn ConstructionScript)