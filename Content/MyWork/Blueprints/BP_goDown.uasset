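; BP_goDown is an actor whose static mesh sinks when the third-person character steps into its box trigger and rises back afterward.
; It saves the mesh's relative transform at BeginPlay as the return pose.
; Begin overlap with the character moves the mesh 200 units down from its current relative location using MoveComponentTo.
; Any end overlap, with no character check, moves it back to the saved location and rotation over half a second.
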(event OnComponentBeginOverlap(Box)
  (params (OverlappedComponent :type Primitive%20Component%20Object%20Reference) (OtherActor :type Actor%20Object%20Reference) (OtherComp :type Primitive%20Component%20Object%20Reference) (OtherBodyIndex :type Integer) (bFromSweep :type Boolean) (SweepResult :type Hit%20Result%20Structure%20%28by%20ref%29))
  (bind _staticmeshcomponent (Variables|Debug|GetStaticMeshComponent))
  (bind _relativelocation (Variables|/Script/Engine.SceneComponent|GetRelativeLocation _staticmeshcomponent))
  (Utilities|Casting|CastToBP_ThirdPersonCharacter OtherActor)
  (Components|MoveComponentTo _staticmeshcomponent (Math|Vector|MakeVector (.x _relativelocation) (.y _relativelocation) (- (.z _relativelocation) 2e+02)) "0, 0, 0" false false 0.2 false))

(event OnComponentEndOverlap(Box)
  (params (OverlappedComponent :type Primitive%20Component%20Object%20Reference) (OtherActor :type Actor%20Object%20Reference) (OtherComp :type Primitive%20Component%20Object%20Reference) (OtherBodyIndex :type Integer))
  (bind _newvar (Variables|Default|GetNewVar))
  (Components|MoveComponentTo (Variables|Debug|GetStaticMeshComponent) (.location _newvar) (.rotation _newvar) false false 0.5 false))

(event EventBeginPlay
  (Variables|Default|SetNewVar (Transformation|GetRelativeTransform (Variables|Debug|GetStaticMeshComponent))))

(event Collision|EventActorBeginOverlap
  (params (OtherActor :type Actor%20Object%20Reference)))

(event EventTick
  (params (DeltaSeconds :type Float%20%28single-precision%29)))

(fn ConstructionScript)